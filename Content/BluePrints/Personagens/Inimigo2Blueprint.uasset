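; Enemy character Blueprint (Inimigo2) that chases the hero, attacks on contact and dies when its health runs out.
; PawnSensing prints a debug message and moves it toward the position of a seen HeroiCaracter.
; Capsule contact with the hero raises IsAtaque for a second, while hits during the hero's kick (IsChute) reduce Vida.
; Tick polls Vida, setting IsMorto and destroying the actor after a delay once it reaches zero.
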(event OnSeePawn(PawnSensing)
  (params (Pawn :type Pawn%20Object%20Reference))
  (Development|PrintString "eu ti vi")
  (bind _asheroi_caracter (Utilities|Casting|CastToHeroiCaracter Pawn))
  (AI|Navigation|SimpleMovetoLocation (Pawn|GetController) (Transformation|GetActorLocation _asheroi_caracter)))

(event OnComponentHit(CapsuleComponent)
  (params (HitComponent :type Primitive%20Component%20Object%20Reference) (OtherActor :type Actor%20Object%20Reference) (OtherComp :type Primitive%20Component%20Object%20Reference) (NormalImpulse :type Vector :default "0, 0, 0") (Hit :type Hit%20Result%20Structure%20%28by%20ref%29))
  (Utilities|Casting|CastToHeroiCaracter OtherActor)
  (Variables|Default|Setis_ataque true)
  (Utilities|FlowControl|Delay 1.0)
  (Variables|Default|Setis_ataque false))

(event Collision|EventHit
  (params (MyComp :type Primitive%20Component%20Object%20Reference) (Other :type Actor%20Object%20Reference) (OtherComp :type Primitive%20Component%20Object%20Reference) (bSelfMoved :type Boolean) (HitLocation :type Vector :default "0, 0, 0") (HitNormal :type Vector :default "0, 0, 0") (NormalImpulse :type Vector :default "0, 0, 0") (Hit :type Hit%20Result%20Structure%20%28by%20ref%29))
  (bind _asheroi_caracter (Utilities|Casting|CastToHeroiCaracter Other))
  (if (Math|Boolean|Equal(Boolean) (Variables|/Game/BluePrints/Personagens/HeroiCaracter.HeroiCaracter_C|Getis_chute _asheroi_caracter) true)
    (Variables|Default|Setvida (- (Variables|Default|Getvida) 1))))

(event EventTick
  (params (DeltaSeconds :type Float%20%28single-precision%29))
  (if (<= (Variables|Default|Getvida) 0)
    (Variables|Default|Setis_morto true)
    (Utilities|FlowControl|Delay 3.0)
    (Actor|DestroyActor)))

(fn ConstructionScript)
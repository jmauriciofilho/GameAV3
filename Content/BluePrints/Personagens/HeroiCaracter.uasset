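; HeroiCaracter is the player hero character, handling movement, camera look, jumping, attacks and an item pickup.
; Axis inputs move it relative to control yaw, while jump, attack and kick inputs toggle state booleans, likely read by animation.
; Both attacks spawn projectiles at an arrow component, but the second works only after a capsule hit on Item1 destroys that item and sets the unlock flag.
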(event OnComponentHit(CapsuleComponent)
  (params (HitComponent :type Primitive%20Component%20Object%20Reference) (OtherActor :type Actor%20Object%20Reference) (OtherComp :type Primitive%20Component%20Object%20Reference) (NormalImpulse :type Vector :default "0, 0, 0") (Hit :type Hit%20Result%20Structure%20%28by%20ref%29))
  (bind _asitem_1 (Utilities|Casting|CastToItem1 OtherActor))
  (Actor|DestroyActor _asitem_1)
  (Variables|Default|Settaken_iten_1 true))

(event Input|ActionEvents|InputActionJump
  (params (Key :type Key%20Structure))
  (:Pressed
    (Character|Jump)
    (Variables|Default|Setis_falling true))
  (:Released
    (Character|StopJumping)
    (Variables|Default|Setis_falling false)))

(event Input|ActionEvents|InputActionAtaque
  (params (Key :type Key%20Structure))
  (:Pressed
    (Variables|Default|Setis_ataque true)
    (Game|SpawnActorfromClass "/Game/BluePrints/Itens/ProjetilBluePrint.ProjetilBluePrint_C" (Transformation|GetWorldTransform (Variables|Default|GetArrow1)) "Undefined" 0 0))
  (:Released
    (Variables|Default|Setis_ataque false)))

(event Input|ActionEvents|InputActionChute
  (params (Key :type Key%20Structure))
  (:Pressed
    (Variables|Default|Setis_chute true))
  (:Released
    (Variables|Default|Setis_chute false)))

(event Input|ActionEvents|InputActionAtaque2
  (params (Key :type Key%20Structure))
  (:Pressed
    (if (Variables|Default|Gettaken_iten_1)
      (Variables|Default|Setis_ataque2 true)
      (Game|SpawnActorfromClass "/Game/BluePrints/Itens/Projetil2Blueprint.Projetil2Blueprint_C" (Transformation|GetWorldTransform (Variables|Default|GetArrow1)) "Undefined" 0 0)))
  (:Released
    (Variables|Default|Setis_ataque2 false)))

(event Input|AxisEvents|InputAxisMoveFoward
  (params (AxisValue :type Float%20%28single-precision%29))
  (Pawn|Input|AddMovementInput (Math|Vector|GetForwardVector (Math|Rotator|MakeRotator 0.0 0.0 (.Yaw (Math|Rotator|BreakRotator (Pawn|GetControlRotation :!class /Script/Engine.Pawn))))) AxisValue false))

(event Input|AxisEvents|InputAxisMoveRight
  (params (AxisValue :type Float%20%28single-precision%29))
  (Pawn|Input|AddMovementInput (Math|Vector|GetRightVector (Math|Rotator|MakeRotator 0.0 0.0 (.Yaw (Math|Rotator|BreakRotator (Pawn|GetControlRotation :!class /Script/Engine.Pawn))))) AxisValue false))

(event Input|AxisEvents|InputAxisTurn
  (params (AxisValue :type Float%20%28single-precision%29))
  (Pawn|Input|AddControllerYawInput AxisValue))

(event Input|AxisEvents|InputAxisLookUpRate
  (params (AxisValue :type Float%20%28single-precision%29))
  (Pawn|Input|AddControllerPitchInput AxisValue))

(fn ConstructionScript)
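; HeroiCaracter is the player-controlled hero character Blueprint, handling movement, camera look, jumping and an attack input.
; Movement axes push the character along forward and right vectors built from control yaw only, while look axes feed controller yaw and pitch.
; Jump starts and stops the jump and toggles IsFalling from the button state rather than actual airborne state.
; The Ataque (attack) action only toggles an IsAtaque flag while held.
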(event Input|ActionEvents|InputActionJump
  (params (Key :type Key%20Structure))
  (:Pressed
    (Character|Jump)
    (Variables|Default|Setis_falling true))
  (:Released
    (Character|StopJumping)
    (Variables|Default|Setis_falling false)))

(event Input|ActionEvents|InputActionAtaque
  (params (Key :type Key%20Structure))
  (:Pressed
    (Variables|Default|Setis_ataque true))
  (:Released
    (Variables|Default|Setis_ataque false)))

(event Input|AxisEvents|InputAxisMoveFoward
  (params (AxisValue :type Float%20%28single-precision%29))
  (Pawn|Input|AddMovementInput (Math|Vector|GetForwardVector (Math|Rotator|MakeRotator 0.0 0.0 (.Yaw (Math|Rotator|BreakRotator (Pawn|GetControlRotation :!class /Script/Engine.Pawn))))) AxisValue false))

(event Input|AxisEvents|InputAxisMoveRight
  (params (AxisValue :type Float%20%28single-precision%29))
  (Pawn|Input|AddMovementInput (Math|Vector|GetRightVector (Math|Rotator|MakeRotator 0.0 0.0 (.Yaw (Math|Rotator|BreakRotator (Pawn|GetControlRotation :!class /Script/Engine.Pawn))))) AxisValue false))

(event Input|AxisEvents|InputAxisTurn
  (params (AxisValue :type Float%20%28single-precision%29))
  (Pawn|Input|AddControllerYawInput AxisValue))

(event Input|AxisEvents|InputAxisLookUpRate
  (params (AxisValue :type Float%20%28single-precision%29))
  (Pawn|Input|AddControllerPitchInput AxisValue))

(fn ConstructionScript)